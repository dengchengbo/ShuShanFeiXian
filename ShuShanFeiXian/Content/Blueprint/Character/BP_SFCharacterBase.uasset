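; BP_SFCharacterBase is a base character Blueprint providing shared movement, mesh registry, combo lookup and empty attack start, reply and end notify events.
; InitEvent fills MeshMap with the skeletal body and static weapon meshes, while Input Movement forwards to AddMovementInput.
; SpeedAnim returns speed normalized by max speed, and ComboInfoList fetches the ComboID's combo list from the SF config manager.
; The weapon-to-hand socket attachment is left unconnected and never runs.
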(event Custom|Input%20Movement
  (params (WorldDirection :type Vector) (ScaleValue :type Float%20%28single-precision%29) (bForce :type Boolean))
  ;[1 1 1] 移动
  (Pawn|Input|AddMovementInput WorldDirection ScaleValue bForce))

(event EventBeginPlay)

(event Collision|EventActorBeginOverlap
  (params (OtherActor :type Actor%20Object%20Reference)))

(event EventTick
  (params (DeltaSeconds :type Float%20%28single-precision%29)))

(event EventInitEvent
  (Utilities|FlowControl|Sequence
    (:then_1
      (CallFunction|InitMeshMap))))

(event EventAttackStartNotifyEvent)

(event EventAttackReplyNotifyEvent)

(event EventAttackEndNotifyEvent)

(fn ConstructionScript)

(fn SpeedAnim
  (return (/ (Math|Vector|VectorLength (Transformation|GetVelocity)) (Class|MovementComponent|GetMaxSpeed (Variables|Character|GetCharacterMovement)))))

(fn InitMeshMap
  (bind _meshmap (Variables|Default|GetMeshMap))
  (Utilities|Map|Add _meshmap "Protagonist" (Utilities|Struct|MakeST_MeshInfo "SkeletalMesh" (Variables|Character|GetMesh)))
  (Utilities|Map|Add _meshmap "Weapon" (Utilities|Struct|MakeST_MeshInfo "StaticMesh" (Variables|Default|GetWeapon))))

(fn ComboInfoList
  (return (.ComboList (Utilities|Struct|BreakComboList (Class|SFConfigManager|GetSFComboInfoPure (Class|SFBPFunction|GetSFConfigManagerPure self) (Variables|Default|GetComboID))))))