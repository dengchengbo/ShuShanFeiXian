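; Player character Blueprint that extends a parent character with equipment setup, mouse-facing attacks and look-relative movement vectors.
; On init it registers the Weapon static mesh with the equipment component and caches its player controller.
; When an attack starts, it snaps the capsule's yaw toward the cursor using a visibility-trace helper.
; A separate event derives 3D forward and right movement vectors from a LookAt input.
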(event Custom|Eve%20Follow%20The%20Mouse
  ;[1 1 1] Comment
  (bind _rotresult (Class|BaseBPFunction|FollowtheMouse self "TraceTypeQuery1" (Transformation|GetActorLocation)))
  (Transformation|SetWorldRotation (Variables|Default|GetCapsuleComponent) (Math|Rotator|MakeRotator 0.0 0.0 (.yaw _rotresult)) false false))

(event Custom|Eve%20According%20Toward
  (params (_LookAt :type Vector))
  ;[1 1 1] Comment
  (Variables|Default|SetSwitchV3 true)
  (bind (__moveforward_3d __moveright_3d) (Class|BaseBPFunction|AccordingToward _LookAt self))
  (Variables|Default|SetMoveForward_3D __moveforward_3d)
  (Variables|Default|SetMoveRight_3D __moveright_3d))

(event EventBeginPlay)

(event Collision|EventActorBeginOverlap
  (params (OtherActor :type Actor%20Object%20Reference)))

(event EventTick
  (params (DeltaSeconds :type Float%20%28single-precision%29)))

(event EventInitEvent
  (|CallParentFunction)
  (Utilities|FlowControl|Sequence
    (:then_0
      (CallFunction|InitEquipment))
    (:then_1
      (bind _asbp_sfplayer_controller (Utilities|Casting|CastToBP_SFPlayerController (Pawn|GetController)))
      (Variables|Default|SetPlayer%20Controller _asbp_sfplayer_controller))))

(event EventAttackStartNotifyEvent
  ;[1 1 1] Comment
  (|CallParentFunction)
  (CallFunction|EveFollowtheMouse))

(fn ConstructionScript
  (|CallParentFunction))

(fn InitEquipment
  (Class|EquipmentComponent|AttachMeshComponenttoInfo (Variables|Default|GetEquipmentComponent) "Weapon" (Variables|Default|GetWeapon) "StaticMesh"))