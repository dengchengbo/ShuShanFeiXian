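; Base NPC character that detects the player and relays combat events to its BP_SFMosterAIController.
; Sight perception or Perception overlap starts the controller's Fighting on a player, then disables both detection methods.
; AttackRange overlaps and attack-end notifies are forwarded to the controller.
; When SwitchV3 is set, Tick applies stored movement inputs along the capsule's forward and right vectors, with a look-at event rotating the capsule toward a target.
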(event OnTargetPerceptionUpdated(Visual)
  (params (Actor :type Actor%20Object%20Reference) (Stimulus :type AI%20Stimulus%20Structure))
  ;[1 1 1] 感知目标
  (if (.bSuccessfullySensed (Utilities|Struct|BreakAIStimulus Stimulus))
    (CallFunction|PerceptionOftheEnemy Actor)))

(event OnComponentBeginOverlap(Perception)
  (params (OverlappedComponent :type Primitive%20Component%20Object%20Reference) (OtherActor :type Actor%20Object%20Reference) (OtherComp :type Primitive%20Component%20Object%20Reference) (OtherBodyIndex :type Integer) (bFromSweep :type Boolean) (SweepResult :type Hit%20Result%20Structure%20%28by%20ref%29))
  ;[1 1 1] 感知目标
  (CallFunction|PerceptionOftheEnemy OtherActor))

(event OnComponentBeginOverlap(AttackRange)
  (params (OverlappedComponent :type Primitive%20Component%20Object%20Reference) (OtherActor :type Actor%20Object%20Reference) (OtherComp :type Primitive%20Component%20Object%20Reference) (OtherBodyIndex :type Integer) (bFromSweep :type Boolean) (SweepResult :type Hit%20Result%20Structure%20%28by%20ref%29))
  ;[1 1 1] Comment
  (Default|RangeOfAttackDeterminationin (Variables|Default|GetAIController) OverlappedComponent OtherActor OtherComp OtherBodyIndex bFromSweep SweepResult))

(event OnComponentEndOverlap(AttackRange)
  (params (OverlappedComponent :type Primitive%20Component%20Object%20Reference) (OtherActor :type Actor%20Object%20Reference) (OtherComp :type Primitive%20Component%20Object%20Reference) (OtherBodyIndex :type Integer))
  ;[1 1 1] Comment
  (Default|RangeOfAttackDeterminationOut (Variables|Default|GetAIController) OverlappedComponent OtherActor OtherComp OtherBodyIndex))

(event Custom|Perception%20of%20the%20enemy
  (params (Actor :type Actor%20Object%20Reference))
  ;[1 1 1] 感知目标
  (bind _asbp_sfplayer_character (Utilities|Casting|CastToBP_SFPlayerCharacter Actor))
  (Utilities|FlowControl|Sequence
    (:then_0
      (Default|Fighting (Variables|Default|GetAIController) _asbp_sfplayer_character))
    (:then_1
      (CallFunction|EnablePerception false))))

(event Custom|LookAtTaget
  (params (Target :type Vector%20%28by%20ref%29))
  ;[1 1 1] Comment
  (Transformation|SetWorldRotation (Variables|Default|GetCapsuleComponent) (Math|Rotator|FindLookatRotation (Transformation|GetActorLocation) Target) false false))

(event Custom|Movement_3D
  (bind _capsulecomponent (Variables|Default|GetCapsuleComponent))
  ;[1 1 1] Comment
  (Utilities|FlowControl|Sequence
    (:then_0
      (CallFunction|InputMovement (Math|Vector|GetForwardVector _capsulecomponent) (Variables|Default|GetMoveUp) false))
    (:then_1
      (CallFunction|InputMovement (Math|Vector|GetRightVector _capsulecomponent) (Variables|Default|GetMoveRight) false))))

(event Custom|Set%20Movement%20State
  (params (MoveUp :type Float%20%28single-precision%29) (MoveRight :type Float%20%28single-precision%29))
  ;[1 1 1] Comment
  (bind _output_get (Variables|Default|SetMoveUp MoveUp))
  (Variables|Default|SetMoveForward_3D _output_get)
  (bind _output_get_2 (Variables|Default|SetMoveRight MoveRight))
  (Variables|Default|SetMoveRight_3D _output_get_2))

(event EventBeginPlay
  (|CallParentFunction) ; This node is disabled and will not be called.\nDrag off pins to build functionality.
)

(event Collision|EventActorBeginOverlap
  (params (OtherActor :type Actor%20Object%20Reference))
  (|CallParentFunction OtherActor) ; This node is disabled and will not be called.\nDrag off pins to build functionality.
)

(event EventTick
  (params (DeltaSeconds :type Float%20%28single-precision%29))
  (|CallParentFunction DeltaSeconds)
  (Utilities|FlowControl|Sequence
    (:then_0
      (if (Variables|Default|GetSwitchV3)
        (CallFunction|Movement3D)))))

(event EventInitEvent
  (bind _asbp_sfmoster_aicontroller (Utilities|Casting|CastToBP_SFMosterAIController (AI|GetAIController self)))
  (Variables|Default|SetAIController _asbp_sfmoster_aicontroller))

(event EventAttackEndNotifyEvent
  ;[1 1 1] Comment
  (|CallParentFunction)
  (Default|IsAttackNeutralBool (Variables|Default|GetAIController) true))

(fn ConstructionScript
  (|CallParentFunction))

(fn EnablePerception
  (params (bEnable :type Boolean))
  (bind _perception (Variables|Default|GetPerception))
  (Utilities|FlowControl|Sequence
    (:then_0
      (Class|AIPerceptionComponent|SetSenseEnabled (Variables|Default|GetVisual) "/Script/AIModule.AISense_Sight" bEnable))
    (:then_1
      (if bEnable
        (Collision|SetCollisionEnabled _perception "QueryOnly")
        (else
          (Collision|SetCollisionEnabled _perception "NoCollision"))))))