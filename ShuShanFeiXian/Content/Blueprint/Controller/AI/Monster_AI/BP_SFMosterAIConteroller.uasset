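; AI controller for SFMonster enemies that drives idle, chase and fighting behaviour against an attack target.
; It runs BT_MosterAI and initialises an ability component, which activates attack and movement abilities by ID.
; Attack-range overlaps and the attack-neutral state are written to Blackboard bools.
; During the five-second attack-neutral window, the monster faces the target, backs off when too close, and uses a looping timer for randomised movement.
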(event Custom|IsAttackNeutral_Bool
  (params (BoolValue :type Boolean))
  ;[1 1 1] 通知是否进入攻击空挡
  (AI|Components|Blackboard|SetValueasBool (AI|GetBlackboard self) (Utilities|Name|MakeLiteralName "IsAttackNeutral") BoolValue))

(event Custom|Action_TakeOff)

(event Custom|Action_Idle)

(event Custom|Action_Attack
  ;[1 1 1] 攻击
  (AI|Navigation|StopMovement)
  (Class|GameplayAbilityComponent|TryActivateAbilitybyID (Variables|Default|GetAbilityComponent) "CM_Attack_1"))

(event Custom|CustomEvent_0
  (bind _returnvalue (Math|Random|RandomFloatinRange -1.0 1.0))
  (bind _returnvalue_2 (* _returnvalue 0.5))
  (bind _returnvalue_3 (> _returnvalue_2 0.1))
  (bind _returnvalue_4 (Math|Float|SelectFloat _returnvalue_2 0.0 _returnvalue_3))
  ;[1 1 1] 攻击空挡
  (if (not (< (Math|Vector|VectorLength (- (Transformation|GetActorLocation (Variables|Default|GetAttackTaget)) (Transformation|GetActorLocation (Variables|Default|GetSFMonster)))) 6e+01))
    (Default|SetMovementState (Variables|Default|GetSFMonster) _returnvalue_4 _returnvalue_4)))

(event Custom|RangeOfAttackDetermination_In
  (params (Overhapped%20Component :type Primitive%20Component%20Object%20Reference) (Other%20Actor :type Actor%20Object%20Reference) (Other%20Comp :type Primitive%20Component%20Object%20Reference) (Other%20Body%20Index :type Integer) (FormSweep :type Boolean) (Sweep%20Result :type Hit%20Result%20Structure))
  ;[1 1 1] Comment
  (if (== Other%20Actor (Variables|Default|GetAttackTaget))
    (CallFunction|SetEnterAttackRangeBool true)))

(event Custom|Action_AttackNeutral
  ;[1 1 1] 攻击空挡
  (Utilities|FlowControl|Sequence
    (:then_0
      (Default|LookatTaget (Variables|Default|GetSFMonster) (Transformation|GetActorLocation (Variables|Default|GetAttackTaget)))
      (AI|Navigation|StopMovement))
    (:then_1
      (Utilities|FlowControl|Delay 5.0)
      (Variables|/Game/Blueprint/Character/BP_SFCharacterBase.BP_SFCharacterBase_C|SetSwitchV3 (Variables|Default|GetSFMonster) false)
      (Utilities|Time|ClearandInvalidateTimerbyHandle (stale _returnvalue))
      (CallFunction|IsAttackNeutralBool false)
      (goto _label Reset))
    (:then_2
      (Variables|/Game/Blueprint/Character/BP_SFCharacterBase.BP_SFCharacterBase_C|SetSwitchV3 (Variables|Default|GetSFMonster) true)
      (Utilities|FlowControl|DoOnce false :!label _label
        (:Completed
          (bind _returnvalue (Utilities|Time|SetTimerbyEvent (delegate Custom|CustomEvent_0) 1.0 true)))))
    (:then_3
      (if (< (Math|Vector|VectorLength (- (Transformation|GetActorLocation (Variables|Default|GetAttackTaget)) (Transformation|GetActorLocation (Variables|Default|GetSFMonster)))) 6e+01)
        (Default|SetMovementState (Variables|Default|GetSFMonster) -0.5 0.0)))))

(event Custom|RangeOfAttackDetermination_Out
  (params (Overhapped%20Component :type Primitive%20Component%20Object%20Reference) (Other%20Actor :type Actor%20Object%20Reference) (Other%20Comp :type Primitive%20Component%20Object%20Reference) (Other%20Body%20Index :type Integer))
  ;[1 1 1] Comment
  (if (== (Variables|Default|GetAttackTaget) Other%20Actor)
    (CallFunction|SetEnterAttackRangeBool false)))

(event Custom|Action_OnHit)

(event Custom|Action_Dead)

(event Custom|SetEnterAttackRange_Bool
  (params (BoolValue :type Boolean))
  ;[1 1 1] 通知是否进入攻击范围
  (AI|Components|Blackboard|SetValueasBool (AI|GetBlackboard self) (Utilities|Name|MakeLiteralName "AttackRange") BoolValue))

(event Custom|Fighting
  (params (AttackTaget :type Actor%20Object%20Reference))
  (Variables|Default|SetAttackTaget AttackTaget)
  (Variables|Default|SetAIAction "Fighting"))

(event Custom|Action_Chase
  ;[1 1 1] 追逐
  (Class|GameplayAbilityComponent|TryActivateAbilitybyID (Variables|Default|GetAbilityComponent) "CM_Move_AI"))

(event EventBeginPlay)

(event EventTick
  (params (DeltaSeconds :type Float%20%28single-precision%29)))

(event EventInit
  ;[1 1 1] 初始化
  (Utilities|FlowControl|Sequence
    (:then_0
      (Variables|Default|SetAIAction "Idle")
      (AI|RunBehaviorTree "/Game/Blueprint/Controller/AI/Monster_AI/BT_MosterAI.BT_MosterAI"))
    (:then_1
      (bind _asbp_sfmonster (Utilities|Casting|CastToBP_SFMonster (Pawn|GetControlledPawn)))
      (bind _output_get (Variables|Default|SetSFMonster _asbp_sfmonster))
      (Class|GameplayAbilityComponent|Init (Variables|Default|GetAbilityComponent) self _output_get))))

(fn ConstructionScript
  (|CallParentFunction))