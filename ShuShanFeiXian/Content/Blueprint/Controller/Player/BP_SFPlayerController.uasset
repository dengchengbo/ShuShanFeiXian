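; Player controller that sets up the player's inventory, ability system and HUD, and routes input to them.
; Init links the controlled pawn to the inventory and ability components, then creates the main UI and a drag-drop layer bound to the inventory.
; Movement axes write to the character, with the up axis triggering a move ability by ID.
; Left click triggers an attack ability; other actions open inventory, pick up items or toggle equipment.
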(event EventBeginPlay)

(event EventTick
  (params (DeltaSeconds :type Float%20%28single-precision%29)))

(event EventInit
  ;[1 1 1] 初始化
  (Utilities|FlowControl|Sequence
    (:then_0
      (bind _asbp_sfplayer_character (Utilities|Casting|CastToBP_SFPlayerCharacter (Pawn|GetControlledPawn)))
      (bind _output_get (Variables|Default|SetPlayerCharacter _asbp_sfplayer_character))
      (Variables|/Game/Blueprint/Component/Inventory/BP_InventoryComponent.BP_InventoryComponent_C|SetCharacter (Variables|Default|GetInventoryComponent) _output_get)
      (Class|GameplayAbilityComponent|Init (Variables|Default|GetAbilityComponent) self _output_get))
    (:then_1
      (bind _returnvalue (UserInterface|CreateWidget "/Game/UI/Convention/UI_Main.UI_Main_C"))
      (bind _output_get_2 (Variables|Default|SetUI_Main _returnvalue))
      (UserInterface|Viewport|AddtoViewport _output_get_2 0)
      (bind _returnvalue_2 (UserInterface|CreateWidget "/Game/UI/Drap/UI_OnDrap_Main.UI_OnDrap_Main_C" 0 (Variables|Default|GetInventoryComponent)))
      (UserInterface|Viewport|AddtoViewport _returnvalue_2 -1))))

(event Input|ActionEvents|InputActionInventory
  (params (Key :type Key%20Structure :default "None"))
  ;[1 1 1] 背包
  (:Pressed
    (Class|InventoryComponent|OpenInventory (Variables|Default|GetInventoryComponent))))

(event Input|ActionEvents|InputActionPickUp
  (params (Key :type Key%20Structure :default "None"))
  ;[1 1 1] 拾取
  (:Pressed
    (Default|InputPickUpItem (Variables|Default|GetInventoryComponent))))

(event Input|ActionEvents|InputActionEquipment
  (params (Key :type Key%20Structure :default "None"))
  (bind _playercharacter (Variables|Default|GetPlayerCharacter))
  (bind _equipmentcomponent (Variables|/Game/Blueprint/Character/Player/BP_SFPlayerCharacter.BP_SFPlayerCharacter_C|GetEquipmentComponent _playercharacter))
  ;[1 1 1] Comment
  (:Pressed
    (Utilities|FlowControl|FlipFlop
      (:A
        (Class|EquipmentComponent|OpenEquipment _equipmentcomponent))
      (:B
        (Class|EquipmentComponent|CloseEquipment _equipmentcomponent)))))

(event Input|AxisEvents|InputAxisMoveUp
  (params (AxisValue :type Float%20%28single-precision%29))
  ;[1 1 1] 移动
  (Variables|/Script/ShuShanFeiXian.SFCharacterBase|SetMoveUp (Variables|Default|GetPlayerCharacter) AxisValue)
  (Class|GameplayAbilityComponent|TryActivateAbilitybyID (Variables|Default|GetAbilityComponent) "CM_Move"))

(event Input|AxisEvents|InputAxisMoveRight
  (params (AxisValue :type Float%20%28single-precision%29))
  ;[1 1 1] 移动
  (Variables|/Script/ShuShanFeiXian.SFCharacterBase|SetMoveRight (Variables|Default|GetPlayerCharacter) AxisValue))

(event Input|MouseEvents|LeftMouseButton
  (params (Key :type Key%20Structure :default "None"))
  ;[1 1 1] temp
  (:Pressed
    (Class|GameplayAbilityComponent|TryActivateAbilitybyID (Variables|Default|GetAbilityComponent) "CM_Attack_1")))

(fn ConstructionScript)