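; BP_RenderTarget2DActor is a stand-in actor in the equipment component folder that mirrors a character's body and weapon meshes.
; On BeginPlay it attaches Weapon to the hand_rWeapon socket and registers both meshes in MeshMap by slot.
; UpdateRender walks a target BP_SFCharacterBase's MeshMap and copies each matching slot's mesh, plus the anim class for skeletal meshes, onto its own components.
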(event Custom|Init
  (Utilities|FlowControl|Sequence
    (:then_0
      (Transformation|AttachComponentToComponent (Variables|Default|GetWeapon) (Variables|Default|GetSkeletalMesh) "hand_rWeapon" "SnapToTarget" "KeepRelative" "KeepRelative" true))
    (:then_1
      (CallFunction|InitMeshMap))))

(event EventBeginPlay
  (CallFunction|Init))

(event Collision|EventActorBeginOverlap
  (params (OtherActor :type Actor%20Object%20Reference)))

(event EventTick
  (params (DeltaSeconds :type Float%20%28single-precision%29)))

(fn ConstructionScript)

(fn UpdateRender
  (params (_Target :type Actor%20Object%20Reference))
  (bind _asbp_sfcharacter_base (Utilities|Casting|CastToBP_SFCharacterBase _Target))
  (bind _keys (Utilities|Map|Keys (Variables|/Game/Blueprint/Character/BP_SFCharacterBase.BP_SFCharacterBase_C|GetMeshMap _asbp_sfcharacter_base)))
  (for _array_element _keys
    (if (.ReturnValue (Utilities|Map|Find (Variables|/Game/Blueprint/Character/BP_SFCharacterBase.BP_SFCharacterBase_C|GetMeshMap _asbp_sfcharacter_base) _array_element))
      (switch Utilities|FlowControl|Switch|SwitchonEGameMeshType (.Type (Utilities|Struct|BreakST_MeshInfo (.Value (Utilities|Map|Find (Variables|/Game/Blueprint/Character/BP_SFCharacterBase.BP_SFCharacterBase_C|GetMeshMap _asbp_sfcharacter_base) _array_element))))
        (:SkeletalMesh
          (bind _asskeletal_mesh_component (Utilities|Casting|CastToSkeletalMeshComponent (.mesh (Utilities|Struct|BreakST_MeshInfo (.Value (Utilities|Map|Find (Variables|/Game/Blueprint/Character/BP_SFCharacterBase.BP_SFCharacterBase_C|GetMeshMap _asbp_sfcharacter_base) _array_element))))))
          (if (.ReturnValue (Utilities|Map|Find (Variables|Default|GetMeshMap) _array_element))
            (bind _asskeletal_mesh_component_2 (Utilities|Casting|CastToSkeletalMeshComponent (.mesh (Utilities|Struct|BreakST_MeshInfo (.Value (Utilities|Map|Find (Variables|Default|GetMeshMap) _array_element))))))
            (Class|SkinnedMeshComponent|SetSkeletalMesh _asskeletal_mesh_component_2 (Variables|/Script/Engine.SkinnedMeshComponent|GetSkeletalMesh _asskeletal_mesh_component) true)
            (Class|SkeletalMeshComponent|SetAnimClass _asskeletal_mesh_component_2 (Variables|/Script/Engine.SkeletalMeshComponent|GetAnimClass _asskeletal_mesh_component))))
        (:StaticMesh
          (bind _asstatic_mesh_component (Utilities|Casting|CastToStaticMeshComponent (.mesh (Utilities|Struct|BreakST_MeshInfo (.Value (Utilities|Map|Find (Variables|/Game/Blueprint/Character/BP_SFCharacterBase.BP_SFCharacterBase_C|GetMeshMap _asbp_sfcharacter_base) _array_element))))))
          (if (.ReturnValue (Utilities|Map|Find (Variables|Default|GetMeshMap) _array_element))
            (bind _asstatic_mesh_component_2 (Utilities|Casting|CastToStaticMeshComponent (.mesh (Utilities|Struct|BreakST_MeshInfo (.Value (Utilities|Map|Find (Variables|Default|GetMeshMap) _array_element))))))
            (Components|StaticMesh|SetStaticMesh _asstatic_mesh_component_2 (Variables|/Script/Engine.StaticMeshComponent|GetStaticMesh _asstatic_mesh_component)))))))
  (return true))

(fn InitMeshMap
  (bind _meshmap (Variables|Default|GetMeshMap))
  (Utilities|Map|Add _meshmap "Protagonist" (Utilities|Struct|MakeST_MeshInfo "SkeletalMesh" (Variables|Default|GetSkeletalMesh)))
  (Utilities|Map|Add _meshmap "Weapon" (Utilities|Struct|MakeST_MeshInfo "StaticMesh" (Variables|Default|GetWeapon))))