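; Inventory component that handles item pickup, throwing and the inventory screen for its owning character.
; Every tick a sphere trace below the character's center caches any hit PickUpActorBase and prints its name, ready for the pickup input.
; Throwing spawns the item's pickup class ahead of the character and launches its mesh forward and up.
; OpenInventory uses a FlipFlop to create or remove the inventory widget, leaving the cursor shown either way.
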(event Custom|Input%20PickUpItem
  (bind _pick_up_actor (Variables|Default|GetPick%20Up%20Actor))
  (Utilities|IsValid _pick_up_actor
    (:Is%20Valid
      (Class|InventoryComponent|PickUpItem _pick_up_actor))))

(event Custom|CheckPickUp
  (bind _character (Variables|Default|GetCharacter))
  (bind _returnvalue (Transformation|GetActorTransform _character))
  (bind _returnvalue_2 (+ (.location _returnvalue) "0, 0,-50.000000"))
  (bind (_outhit _returnvalue_3) (Collision|SphereTraceForObjects _returnvalue_2 _returnvalue_2 1e+02 (Utilities|Array|MakeArray "ObjectTypeQuery7") false 0 "None"))
  (if _returnvalue_3
    (bind _aspick_up_actor_base (Utilities|Casting|CastToPickUpActorBase (.HitActor (Collision|BreakHitResult _outhit)))
      (:then
        (bind _output_get (Variables|Default|SetPick%20Up%20Actor _aspick_up_actor_base))
        (Development|PrintText (Utilities|Text|ToText(String) (Utilities|GetDisplayName _output_get)) true true "(R=0.000000,G=0.660000,B=1.000000,A=1.000000)" 0.0))
      (:CastFailed
        (Variables|Default|SetPick%20Up%20Actor 0 :!label _label)))
    (else
      (goto _label))))

(event Custom|Input%20ThrowItem
  (params (_Index :type Integer) (_Num :type Integer))
  (Class|InventoryComponent|ThrowItem _Index _Num))

(event EventBeginPlay)

(event EventTick
  (params (DeltaSeconds :type Float%20%28single-precision%29))
  (CallFunction|CheckPickUp))

(event EventThrowItemEvent
  (params (_Info :type Item%20Info%20Structure))
  (bind _character (Variables|Default|GetCharacter))
  (bind _returnvalue (Transformation|GetActorTransform _character))
  (bind _returnvalue_2 (Transformation|GetActorForwardVector _character))
  (bind _returnvalue_3 (Game|SpawnActorfromClass (.PickUpActorBaseClass (Utilities|Struct|BreakItemInfo _Info)) (Math|Transform|MakeTransform (+ (.location _returnvalue) (* _returnvalue_2 2e+01)) (.rotation _returnvalue) "1,1,1") "Undefined" 0 _Info 0))
  (Physics|SetPhysicsLinearVelocity (Variables|/Script/InventoryModule.PickUpActorBase|GetStaticMesh _returnvalue_3) (* (+ _returnvalue_2 "0, 0,1.000000") 1.5e+02) false "None"))

(event EventOpenInventory
  (bind _returnvalue (Game|GetPlayerController 0))
  ;[1 1 1] 打开背包
  (Utilities|FlowControl|FlipFlop
    (:A
      (bind _returnvalue_2 (UserInterface|CreateWidget "/Game/UI/Inventory/UI_Inventory_Main.UI_Inventory_Main_C" 0 (Class|InventoryComponent|GetInventory) self))
      (bind _output_get (Variables|Default|SetUI_Inventory _returnvalue_2))
      (UserInterface|Viewport|AddtoViewport _output_get 0)
      (Variables|/Script/Engine.PlayerController|SetbShowMouseCursor _returnvalue true))
    (:B
      (Widget|RemovefromParent (Variables|Default|GetUI_Inventory))
      (Variables|/Script/Engine.PlayerController|SetbShowMouseCursor _returnvalue true))))